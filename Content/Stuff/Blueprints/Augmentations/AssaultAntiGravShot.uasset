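; Assault augmentation that fires an anti-gravity projectile from the first-person player when used, gated by a cooldown.
; Tick counts the cooldown down by delta time, and OnUse fires only once it reaches zero, then resets it to the wait penalty.
; The shot spawns at the pistol sphere plus a camera-rotated pistol offset, facing the camera direction, with gunfire sound and a muzzle emitter on the assault sphere.
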(event `self.ReceiveBeginPlay`
  (bind _asfirst_person_character (cast `/Game/FirstPersonBP/Blueprints/FirstPersonCharacter` (`GameplayStatics.GetPlayerCharacter` 0)))
  (set `self.Player` _asfirst_person_character))

(event `self.ReceiveTick`
  (params (DeltaSeconds :type "Float (single-precision)"))
  (set `self.AlterValue` DeltaSeconds)
  (if (not (<= (`self.Cooldown`) 0.0))
    (`self.refill cooldown`)))

(event `/Game/Stuff/Blueprints/Augmentations/Augment.OnUse`
  (if (<= (`self.Cooldown`) 0.0)
    (`self.FireAntiGravShot`)
    (set `self.Cooldown` (`self.WaitPenalty`))))

(fn `FireAntiGravShot`
  (bind _player (`self.Player`))
  (bind _transformation (`self.GetTransformation`))
  (`|SpawnActorFromClass` "/Game/Stuff/Blueprints/Bullets/AntiGravityShot.AntiGravityShot_C" _transformation "AdjustIfPossibleButDontSpawnIfColliding" "OverrideRootScale" null null) ; Spawn projectile
  (`GameplayStatics.PlaySoundAtLocation` "/Game/Stuff/Sounds/AK47_SoundEffect.AK47_SoundEffect" (`Actor.K2_GetActorLocation` _player) (struct) (`/Game/FirstPersonBP/Blueprints/FirstPersonCharacter.GunVolume` _player)) ; Play firing sound
  (`GameplayStatics.SpawnEmitterAttached` "/Game/StarterContent/Particles/MF_Particle.MF_Particle" (`/Game/FirstPersonBP/Blueprints/FirstPersonCharacter.AssaultSphere` _player)))

(fn `GetTransformation`
  (returns (Transformation :type "Transform Structure"))
  (bind _player (`self.Player`))
  (bind _returnvalue (`SceneComponent.K2_GetComponentRotation` (`/Game/FirstPersonBP/Blueprints/FirstPersonCharacter.FirstPersonCamera` _player)))
  (return (`KismetMathLibrary.MakeTransform` (+ (`SceneComponent.K2_GetComponentLocation` (`/Game/FirstPersonBP/Blueprints/FirstPersonCharacter.PistolSphere` _player)) (`KismetMathLibrary.GreaterGreater_VectorRotator` (`/Game/FirstPersonBP/Blueprints/FirstPersonCharacter.PistolOffset` _player) _returnvalue)) _returnvalue (0.5 0.5 0.5))))

(fn `refill cooldown`
  (set `self.Cooldown` (- (`self.Cooldown`) (`self.AlterValue`))))