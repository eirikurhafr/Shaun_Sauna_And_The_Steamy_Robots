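; Slow-motion augmentation that toggles global time dilation on use, slowing the world to a fifth of normal speed.
; Tick drains an energy bar while active and refills it up to full while inactive.
; An empty bar automatically restores normal time.
; Bar changes are fixed per-tick steps, not scaled by delta time, and the player character is cached on BeginPlay.
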(event `self.ReceiveBeginPlay`
  (bind _asfirst_person_character (cast `/Game/FirstPersonBP/Blueprints/FirstPersonCharacter` (`GameplayStatics.GetPlayerCharacter` 0)))
  (set `self.Player` _asfirst_person_character))

(event `self.ReceiveTick`
  (params (DeltaSeconds :type "Float (single-precision)"))
  (if (`self.bActivated`)
    (`self.IsActivated`)
    (else
      (`self.IsNotActivated`))))

(event `/Game/Stuff/Blueprints/Augmentations/Augment.OnUse`
  (if (`self.bActivated`)
    (`self.DeactivateSlowMotion`)
    (else
      (`self.ActivateSlowMotion`))))

(fn `ActivateSlowMotion`
  (set `self.bActivated` true)
  (`GameplayStatics.SetGlobalTimeDilation` 0.2))

(fn `DeactivateSlowMotion`
  (set `self.bActivated` false)
  (`GameplayStatics.SetGlobalTimeDilation` 1.0))

(fn `IsActivated`
  (set `self.BarValue` (- (`self.BarValue`) (`self.DecrementValue`)))
  (if (<= (`self.BarValue`) 0.0)
    (`self.DeactivateSlowMotion`)
    (set `self.BarValue` 0.0)))

(fn `IsNotActivated`
  (if (>= (`self.BarValue`) 1.0)
    (set `self.BarValue` 1.0)
    (else
      (set `self.BarValue` (+ (`self.BarValue`) (`self.IncreaseValue`))))))