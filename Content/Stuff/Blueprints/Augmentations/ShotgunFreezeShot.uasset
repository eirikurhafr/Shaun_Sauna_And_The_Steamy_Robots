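; Shotgun freeze-shot augmentation that, on use, fires a spread of FreezeRound projectiles from the player's shotgun, then starts a cooldown.
; Each projectile spawns from the shotgun sphere along the camera rotation with random pitch and yaw jitter, the yaw range scaling with bullet count, plus an attached muzzle particle.
; Tick counts the cooldown down, and Convert exposes it as normalized recharge progress.
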(event `self.ReceiveBeginPlay`
  (bind _asfirst_person_character (cast `/Game/FirstPersonBP/Blueprints/FirstPersonCharacter` (`GameplayStatics.GetPlayerCharacter` 0)))
  (set `self.Player` _asfirst_person_character))

(event `self.ReceiveTick`
  (params (DeltaSeconds :type "Float (single-precision)"))
  (set `self.alter value` DeltaSeconds)
  (if (not (<= (`self.Cooldown`) 0.0))
    (`self.RefillCooldown`)))

(event `/Game/Stuff/Blueprints/Augmentations/Augment.OnUse`
  (if (<= (`self.Cooldown`) 0.0)
    (`self.FireFreezeBullets`)
    (set `self.Cooldown` (`self.Wait Penalty`))))

(fn `Convert`
  (returns (Percentage :type "Float (double-precision)"))
  (return (- 1.0 (/ (`self.Cooldown`) (`self.Wait Penalty`)))))

(fn `FireFreezeBullets`
  (for _ (range (+ (`KismetMathLibrary.FTrunc` (`self.Bullets`)) 1))
    (bind _transform (`self.GetTransformation`))
    (`|SpawnActorFromClass` "/Game/Stuff/Blueprints/Bullets/FreezeRound.FreezeRound_C" _transform "AdjustIfPossibleButDontSpawnIfColliding" "OverrideRootScale" null null) ; Spawn projectile
    (`GameplayStatics.SpawnEmitterAttached` "/Game/StarterContent/Particles/MF_Particle.MF_Particle" (`/Game/FirstPersonBP/Blueprints/FirstPersonCharacter.ShotgunSphere` (`self.Player`)) "None" (0.0 0.0 0.0) (struct) (0.5 0.5 0.5))))

(fn `GetTransformation`
  (returns (Transform :type "Transform Structure"))
  (bind _player (`self.Player`))
  (bind _returnvalue (/ (`self.Bullets`) 2.0))
  (bind _returnvalue_2 (`KismetMathLibrary.MakeRotator` (.roll (`SceneComponent.K2_GetComponentRotation` (`/Game/FirstPersonBP/Blueprints/FirstPersonCharacter.FirstPersonCamera` _player))) (+ (`KismetMathLibrary.RandomFloatInRange` -7.0 7.0) (.pitch (`SceneComponent.K2_GetComponentRotation` (`/Game/FirstPersonBP/Blueprints/FirstPersonCharacter.FirstPersonCamera` _player)))) (+ (.yaw (`SceneComponent.K2_GetComponentRotation` (`/Game/FirstPersonBP/Blueprints/FirstPersonCharacter.FirstPersonCamera` _player))) (`KismetMathLibrary.RandomFloatInRange` (- 0.0 _returnvalue) _returnvalue))))
  (return (`KismetMathLibrary.MakeTransform` (+ (`SceneComponent.K2_GetComponentLocation` (`/Game/FirstPersonBP/Blueprints/FirstPersonCharacter.ShotgunSphere` _player)) (`KismetMathLibrary.GreaterGreater_VectorRotator` (`/Game/FirstPersonBP/Blueprints/FirstPersonCharacter.ShotgunOffset` _player) _returnvalue_2)) _returnvalue_2 (`self.Size`))))

(fn `RefillCooldown`
  (set `self.Cooldown` (- (`self.Cooldown`) (`self.alter value`))))