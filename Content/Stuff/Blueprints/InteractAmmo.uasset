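; Interactable ammo crate pickup that refills the player's reserve ammo for every weapon type.
; On interact, it adds one full magazine to assault, RPG, shotgun and pistol totals, each clamped to that weapon's maximum.
; It then destroys itself and clears HasCrate on its Spawner to mark it empty.
; Each weapon has its own near-identical function that casts player 0 to FirstPersonCharacter.
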(event `/Game/Stuff/Blueprints/Interact/InteractInterface.OnInteract`
  (`self.GiveAmmo`)
  (`self.K2_DestroyActor`)
  (set `/Game/SteamyRobots/PickupSpawners/LootBoxSpawner.HasCrate` false (`self.Spawner`)))

(fn `GiveAmmo`
  (`self.GiveAssaultAmmo`)
  (`self.GiveRPGAmmo`)
  (`self.GiveShotgunAmmo`)
  (`self.GivePistolAmmo`))

(fn `GiveAssaultAmmo`
  (bind _asfirst_person_character (cast `/Game/FirstPersonBP/Blueprints/FirstPersonCharacter` (`GameplayStatics.GetPlayerCharacter` 0)))
  (bind _returnvalue (+ (`/Game/FirstPersonBP/Blueprints/FirstPersonCharacter.AssaultTotalAmmo` _asfirst_person_character) (`/Game/FirstPersonBP/Blueprints/FirstPersonCharacter.AssaultMaxMagAmmo` _asfirst_person_character)))
  (bind _assaultmaxtotalammo (`/Game/FirstPersonBP/Blueprints/FirstPersonCharacter.AssaultMaxTotalAmmo` _asfirst_person_character))
  (if (> _returnvalue _assaultmaxtotalammo)
    (set `/Game/FirstPersonBP/Blueprints/FirstPersonCharacter.AssaultTotalAmmo` _assaultmaxtotalammo _asfirst_person_character)
    (else
      (set `/Game/FirstPersonBP/Blueprints/FirstPersonCharacter.AssaultTotalAmmo` _returnvalue _asfirst_person_character))))

(fn `GivePistolAmmo`
  (bind _asfirst_person_character (cast `/Game/FirstPersonBP/Blueprints/FirstPersonCharacter` (`GameplayStatics.GetPlayerCharacter` 0)))
  (bind _returnvalue (+ (`/Game/FirstPersonBP/Blueprints/FirstPersonCharacter.PistolTotalAmmo` _asfirst_person_character) (`/Game/FirstPersonBP/Blueprints/FirstPersonCharacter.PistolMaxMagAmmo` _asfirst_person_character)))
  (bind _pistolmaxtotalammo (`/Game/FirstPersonBP/Blueprints/FirstPersonCharacter.PistolMaxTotalAmmo` _asfirst_person_character))
  (if (> _returnvalue _pistolmaxtotalammo)
    (set `/Game/FirstPersonBP/Blueprints/FirstPersonCharacter.PistolTotalAmmo` _pistolmaxtotalammo _asfirst_person_character)
    (else
      (set `/Game/FirstPersonBP/Blueprints/FirstPersonCharacter.PistolTotalAmmo` _returnvalue _asfirst_person_character))))

(fn `GiveRPGAmmo`
  (bind _asfirst_person_character (cast `/Game/FirstPersonBP/Blueprints/FirstPersonCharacter` (`GameplayStatics.GetPlayerCharacter` 0)))
  (bind _returnvalue (+ (`/Game/FirstPersonBP/Blueprints/FirstPersonCharacter.RPGTotalAmmo` _asfirst_person_character) (`/Game/FirstPersonBP/Blueprints/FirstPersonCharacter.RPGMaxMagAmmo` _asfirst_person_character)))
  (bind _rpgmaxtotalammo (`/Game/FirstPersonBP/Blueprints/FirstPersonCharacter.RPGMaxTotalAmmo` _asfirst_person_character))
  (if (> _returnvalue _rpgmaxtotalammo)
    (set `/Game/FirstPersonBP/Blueprints/FirstPersonCharacter.RPGTotalAmmo` _rpgmaxtotalammo _asfirst_person_character)
    (else
      (set `/Game/FirstPersonBP/Blueprints/FirstPersonCharacter.RPGTotalAmmo` _returnvalue _asfirst_person_character))))

(fn `GiveShotgunAmmo`
  (bind _asfirst_person_character (cast `/Game/FirstPersonBP/Blueprints/FirstPersonCharacter` (`GameplayStatics.GetPlayerCharacter` 0)))
  (bind _returnvalue (+ (`/Game/FirstPersonBP/Blueprints/FirstPersonCharacter.ShotgunTotalAmmo` _asfirst_person_character) (`/Game/FirstPersonBP/Blueprints/FirstPersonCharacter.ShotgunMaxMagAmmo` _asfirst_person_character)))
  (bind _shotgunmaxtotalammo (`/Game/FirstPersonBP/Blueprints/FirstPersonCharacter.ShotgunMaxTotalAmmo` _asfirst_person_character))
  (if (> _returnvalue _shotgunmaxtotalammo)
    (set `/Game/FirstPersonBP/Blueprints/FirstPersonCharacter.ShotgunTotalAmmo` _shotgunmaxtotalammo _asfirst_person_character)
    (else
      (set `/Game/FirstPersonBP/Blueprints/FirstPersonCharacter.ShotgunTotalAmmo` _returnvalue _asfirst_person_character))))

(fn `UserConstructionScript`)