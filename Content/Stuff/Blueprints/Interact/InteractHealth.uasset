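; InteractHealth is an interactable health pickup that heals the player when used.
; On interact, it calls GiveHealth and then destroys itself.
; GiveHealth casts player character 0 to FirstPersonCharacter and adds a fixed amount to CurrentHealth, or sets it to MaxHealth once health reaches a hard-coded threshold.
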(event `/Game/Stuff/Blueprints/Interact/InteractInterface.OnInteract`
  (`self.GiveHealth`)
  (`self.K2_DestroyActor`))

(fn `GiveHealth`
  (bind _asfirst_person_character (cast `/Game/FirstPersonBP/Blueprints/FirstPersonCharacter` (`GameplayStatics.GetPlayerCharacter` 0)))
  (bind _currenthealth (`/Game/FirstPersonBP/Blueprints/FirstPersonCharacter.CurrentHealth` _asfirst_person_character))
  (if (< _currenthealth 80)
    (set `/Game/FirstPersonBP/Blueprints/FirstPersonCharacter.CurrentHealth` (+ _currenthealth 20) _asfirst_person_character)
    (else
      (set `/Game/FirstPersonBP/Blueprints/FirstPersonCharacter.CurrentHealth` (`/Game/FirstPersonBP/Blueprints/FirstPersonCharacter.MaxHealth` _asfirst_person_character) _asfirst_person_character))))

(fn `UserConstructionScript`)