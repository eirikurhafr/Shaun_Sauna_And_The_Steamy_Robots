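; InteractHealth is an interactable health pickup, tied to a crate spawner, that restores the shrine rather than the player.
; On interact it adds a fixed amount to ShrineHealth on the BPAttackPoint held by FirstPersonGameMode, with no upper clamp.
; It then destroys itself and clears the HasCrate flag on its Spawner.
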(event `/Game/Stuff/Blueprints/Interact/InteractInterface.OnInteract`
  (`self.GiveHealth`)
  (`self.K2_DestroyActor`)
  (set `/Game/SteamyRobots/PickupSpawners/LootBoxSpawner.HasCrate` false (`self.Spawner`)))

(fn `GiveHealth`
  (bind _asfirst_person_game_mode (cast `/Game/FirstPersonBP/Blueprints/FirstPersonGameMode` (`GameplayStatics.GetGameMode`)))
  (bind _bpattackpoint (`/Game/FirstPersonBP/Blueprints/FirstPersonGameMode.BPAttackPoint` _asfirst_person_game_mode))
  (set `/Game/Stuff/Blueprints/AttackPoint.ShrineHealth` (+ (`/Game/Stuff/Blueprints/AttackPoint.ShrineHealth` _bpattackpoint) 25) _bpattackpoint))

(fn `UserConstructionScript`)