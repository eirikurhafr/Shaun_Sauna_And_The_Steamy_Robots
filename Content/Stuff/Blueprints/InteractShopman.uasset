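; Interactable shopkeeper actor that opens the shop UI when the player interacts with it.
; OnInteract calls ActivateShop, which creates the ShopmanInterface widget on first use, caches it as ReferenceHUD and re-adds that same widget on later visits.
; Opening the shop switches input to UI-only and shows the mouse cursor.
; On first creation it also stores itself as ShopManReference on the FirstPersonCharacter.
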(event `/Game/Stuff/Blueprints/InteractInterface.OnInteract`
  (`self.ActivateShop`))

(fn `ActivateShop`
  (bind _returnvalue (`GameplayStatics.GetPlayerController` 0))
  (bind _referencehud (`self.ReferenceHUD`))
  (if (`KismetSystemLibrary.IsValid` (`self.ReferenceHUD`))
    (`WidgetBlueprintLibrary.SetInputMode_UIOnlyEx` _returnvalue _referencehud)
    (`UserWidget.AddToViewport` _referencehud 0)
    (set `PlayerController.bShowMouseCursor` true _returnvalue)
    (else
      (bind _returnvalue_2 (`|CreateWidget` "/Game/Stuff/Widgets/ShopmanInterface.ShopmanInterface_C" _returnvalue))
      (`WidgetBlueprintLibrary.SetInputMode_UIOnlyEx` _returnvalue _returnvalue_2)
      (`UserWidget.AddToViewport` _returnvalue_2 0)
      (set `PlayerController.bShowMouseCursor` true _returnvalue)
      (set `self.ReferenceHUD` _returnvalue_2)
      (bind _asfirst_person_character (cast `/Game/FirstPersonBP/Blueprints/FirstPersonCharacter` (`GameplayStatics.GetPlayerCharacter` 0)))
      (set `/Game/FirstPersonBP/Blueprints/FirstPersonCharacter.ShopManReference` self _asfirst_person_character))))

(fn `UserConstructionScript`)