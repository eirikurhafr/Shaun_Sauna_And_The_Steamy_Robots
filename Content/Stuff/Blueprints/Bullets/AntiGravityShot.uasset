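; Anti-gravity projectile that bursts on contact and activates anti-gravity on bots caught in the blast.
; Its collision overlap ignores the first-person character, other anti-gravity shots and ranged bot rounds; otherwise it enables the Explosion overlap volume, spawns particles and sound, and destroys the Sphere.
; Explosion overlaps call ActivateAntiGravity on melee, ranged and sauna melee bots, the last reached by cast alone because its class check is unwired.
; The Explosion volume is never switched off here.
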(event `self.ReceiveBeginPlay`
  (`PrimitiveComponent.SetCollisionEnabled` (`self.Explosion`) "NoCollision"))

(event `self.CollisionComponent.OnComponentBeginOverlap`
  (params (OverlappedComponent :type "PrimitiveComponent Object Reference") (OtherActor :type "Actor Object Reference") (OtherComp :type "PrimitiveComponent Object Reference") (OtherBodyIndex :type Integer) (bFromSweep :type Boolean) (SweepResult :type "HitResult Structure (by ref)"))
  (bind _returnvalue (`GameplayStatics.GetObjectClass` OtherActor))
  (bind _returnvalue_2 (`SceneComponent.K2_GetComponentLocation` (`self.Sphere`)))
  (if (== _returnvalue "/Game/FirstPersonBP/Blueprints/FirstPersonCharacter.FirstPersonCharacter_C")
    _
    (elif (== _returnvalue "AntiGravityShot_C")
      _
      (elif (not (== _returnvalue "/Game/FirstPersonBP/Blueprints/rangeBotRound.rangeBotRound_C"))
        (`PrimitiveComponent.SetCollisionEnabled` (`self.Explosion`) "QueryOnly")
        (`GameplayStatics.SpawnEmitterAtLocation` "/Game/Stuff/Particle/Enemies/P_AntiGrav.P_AntiGrav" _returnvalue_2 (struct) (4.0 4.0 4.0))
        (`GameplayStatics.SpawnSoundAtLocation` "/Game/Stuff/Sounds/EnergyWhip.EnergyWhip" _returnvalue_2 (struct) 1.0 1.0 0.0 "/Game/NewSoundAttenuation.NewSoundAttenuation")
        (`ActorComponent.K2_DestroyComponent` (`self.Sphere`))))))

(event `self.Explosion.OnComponentBeginOverlap`
  (params (OverlappedComponent :type "PrimitiveComponent Object Reference") (OtherActor :type "Actor Object Reference") (OtherComp :type "PrimitiveComponent Object Reference") (OtherBodyIndex :type Integer) (bFromSweep :type Boolean) (SweepResult :type "HitResult Structure (by ref)"))
  (bind _returnvalue (`GameplayStatics.GetObjectClass` OtherActor))
  (if (== _returnvalue "/Game/SteamyRobots/Ai-stuff/MeleBotBP.MeleBotBP_C")
    (bind _asmele_bot_bp (cast `/Game/SteamyRobots/Ai-stuff/MeleBotBP` OtherActor))
    (`/Game/SteamyRobots/Ai-stuff/MeleBotBP.ActivateAntiGravity` _asmele_bot_bp)
    (elif (== _returnvalue "/Game/SteamyRobots/RangedBots/RangedBot.RangedBot_C")
      (bind _asranged_bot (cast `/Game/SteamyRobots/RangedBots/RangedBot` OtherActor))
      (`/Game/SteamyRobots/RangedBots/RangedBot.ActivateAntiGravity` _asranged_bot)
      (elif true
        (bind _assauna_melee_bot_bp (cast `/Game/Stuff/Bots/ShrineMelee/SaunaMeleeBotBP` OtherActor))
        (`/Game/Stuff/Bots/ShrineMelee/SaunaMeleeBotBP.ActivateAntiGravity` _assauna_melee_bot_bp)))))

(fn `UserConstructionScript`)