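; FreezeRound is a bullet Blueprint that damages enemy bots on overlap, with no freeze effect in its graph.
; Its collision overlap checks the other actor's exact class and calls HurtFunction on MeleBotBP or RangedBot, dealing far more damage to RangedBot.
; A hit spawns the P_HitEnemy emitter at the sphere's location and destroys the round.
; A SaunaMeleeBotBP damage branch exists but is disconnected and never runs.
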(event `self.CollisionComponent.OnComponentBeginOverlap`
  (params (OverlappedComponent :type "PrimitiveComponent Object Reference") (OtherActor :type "Actor Object Reference") (OtherComp :type "PrimitiveComponent Object Reference") (OtherBodyIndex :type Integer) (bFromSweep :type Boolean) (SweepResult :type "HitResult Structure (by ref)"))
  (bind _returnvalue (`GameplayStatics.GetObjectClass` OtherActor))
  (if (== _returnvalue "/Game/SteamyRobots/Ai-stuff/MeleBotBP.MeleBotBP_C")
    (bind _asmele_bot_bp (cast `/Game/SteamyRobots/Ai-stuff/MeleBotBP` OtherActor))
    (`/Game/SteamyRobots/Ai-stuff/MeleBotBP.HurtFunction` _asmele_bot_bp 5)
    (`GameplayStatics.SpawnEmitterAtLocation` "/Game/Stuff/Particle/Shots/P_HitEnemy.P_HitEnemy" (`SceneComponent.K2_GetComponentLocation` (`self.Sphere`)) :!label _label)
    (`self.K2_DestroyActor`)
    (elif (== _returnvalue "/Game/SteamyRobots/RangedBots/RangedBot.RangedBot_C")
      (bind _asranged_bot (cast `/Game/SteamyRobots/RangedBots/RangedBot` OtherActor))
      (`/Game/SteamyRobots/RangedBots/RangedBot.HurtFunction` _asranged_bot 80)
      (goto _label))))

(fn `UserConstructionScript`)