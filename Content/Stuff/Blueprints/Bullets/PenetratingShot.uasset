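; Penetrating bullet that deals fixed damage to melee, ranged and sauna melee bots it overlaps.
; Each overlap runs a per-class check, then hurts the bot, records it in that class's array and spawns a hit emitter.
; The checks do not block repeat hits: melee always passes, while ranged and sauna pass only bots already recorded, so those never get damaged.
; A player-pistol beam emitter chain is left unconnected.
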(event `self.ReceiveBeginPlay`)

(event `self.CollisionComponent.OnComponentBeginOverlap`
  (params (OverlappedComponent :type "PrimitiveComponent Object Reference") (OtherActor :type "Actor Object Reference") (OtherComp :type "PrimitiveComponent Object Reference") (OtherBodyIndex :type Integer) (bFromSweep :type Boolean) (SweepResult :type "HitResult Structure (by ref)"))
  (bind _returnvalue (`GameplayStatics.GetObjectClass` OtherActor))
  (if (== _returnvalue "/Game/SteamyRobots/Ai-stuff/MeleBotBP.MeleBotBP_C")
    (bind _asmele_bot_bp (cast `/Game/SteamyRobots/Ai-stuff/MeleBotBP` OtherActor))
    (bind _alreadyshot (`self.CheckForMelee` _asmele_bot_bp))
    (if _alreadyshot
      (`/Game/SteamyRobots/Ai-stuff/MeleBotBP.HurtFunction` _asmele_bot_bp 25)
      (`KismetArrayLibrary.Array_Add` (`self.MeleeBotArray`) _asmele_bot_bp)
      (`GameplayStatics.SpawnEmitterAtLocation` "/Game/Stuff/Particle/Shots/P_HitEnemy.P_HitEnemy" (`SceneComponent.K2_GetComponentLocation` (`self.Sphere`)) :!label _label))
    (elif (== _returnvalue "/Game/SteamyRobots/RangedBots/RangedBot.RangedBot_C")
      (bind _asranged_bot (cast `/Game/SteamyRobots/RangedBots/RangedBot` OtherActor))
      (bind _alreadyshot_2 (`self.CheckForRanged` _asranged_bot))
      (if _alreadyshot_2
        (`/Game/SteamyRobots/RangedBots/RangedBot.HurtFunction` _asranged_bot 25)
        (`KismetArrayLibrary.Array_Add` (`self.RangedBotArray`) _asranged_bot)
        (goto _label))
      (elif (== _returnvalue "/Game/Stuff/Bots/ShrineMelee/SaunaMeleeBotBP.SaunaMeleeBotBP_C")
        (bind _assauna_melee_bot_bp (cast `/Game/Stuff/Bots/ShrineMelee/SaunaMeleeBotBP` OtherActor))
        (bind _alreadyshot_3 (`self.CheckForMeleeSauna` _assauna_melee_bot_bp))
        (if _alreadyshot_3
          (`/Game/Stuff/Bots/ShrineMelee/SaunaMeleeBotBP.HurtFunction` _assauna_melee_bot_bp 25)
          (`KismetArrayLibrary.Array_Add` (`self.SaunaMeleeBotArray`) _assauna_melee_bot_bp)
          (goto _label))))))

(fn `CheckForMelee`
  (params (Bot :type "/Game/SteamyRobots/Ai-stuff/MeleBotBP Object Reference"))
  (returns (AlreadyShot :type Boolean))
  (for _array_element (`self.MeleeBotArray`)
    (if (== Bot _array_element)
      (return true)))
  (return true))

(fn `CheckForMeleeSauna`
  (params (Bot :type "/Game/Stuff/Bots/ShrineMelee/SaunaMeleeBotBP Object Reference"))
  (returns (AlreadyShot :type Boolean))
  (for _array_element (`self.SaunaMeleeBotArray`)
    (if (== Bot _array_element)
      (return true)))
  (return false))

(fn `CheckForRanged`
  (params (Bot :type "/Game/SteamyRobots/RangedBots/RangedBot Object Reference"))
  (returns (AlreadyShot :type Boolean))
  (for _array_element (`self.RangedBotArray`)
    (if (== Bot _array_element)
      (return true)))
  (return false))

(fn `UserConstructionScript`)