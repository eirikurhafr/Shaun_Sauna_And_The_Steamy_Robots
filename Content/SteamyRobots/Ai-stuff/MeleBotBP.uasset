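; Melee enemy bot for wave combat that damages the player through a sword collider toggled during attacks.
; HurtFunction subtracts health and, at zero, awards currency, updates the wave spawner's alive counts and removes the bot.
; Freeze pauses animation and AI logic with a material swap; anti-gravity lifts the bot into mesh physics simulation.
; Tick-driven Delays end both effects after player-defined durations, and BeginPlay briefly cycles anti-gravity on and off.
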(event `self.ReceiveBeginPlay`
  (set `self.IsAlive` true)
  (`self.ActivateAntiGravity`)
  (`KismetSystemLibrary.Delay` 0.1)
  (`self.DeactivateAntiGravity`)
  (bind _asfirst_person_character (cast `/Game/FirstPersonBP/Blueprints/FirstPersonCharacter` (`GameplayStatics.GetPlayerCharacter` 0)))
  (set `self.Player` _asfirst_person_character))

(event `EnableWeaponTrigger`
  ;[1 1 1] Acctivate and deacctivate weapon collider on attack
  (`PrimitiveComponent.SetCollisionEnabled` (`self.Sword`) "QueryOnly"))

(event `self.ReceiveTick`
  (params (DeltaSeconds :type "Float (single-precision)"))
  (bind _player (`self.Player`))
  (if (`self.Frozen`)
    (`KismetSystemLibrary.Delay` (`/Game/FirstPersonBP/Blueprints/FirstPersonCharacter.FreezeDuration` _player))
    (`self.DeactivateFreeze`)
    (elif (`self.AntiGravity`)
      (`KismetSystemLibrary.Delay` (`/Game/FirstPersonBP/Blueprints/FirstPersonCharacter.AntiGravDuration` _player))
      (`self.DeactivateAntiGravity`))))

(event `DisableWeaponTrigger`
  ;[1 1 1] Acctivate and deacctivate weapon collider on attack
  (`PrimitiveComponent.SetCollisionEnabled` (`self.Sword`) "NoCollision"))

(event `self.Sword.OnComponentBeginOverlap`
  (params (OverlappedComponent :type "PrimitiveComponent Object Reference") (OtherActor :type "Actor Object Reference") (OtherComp :type "PrimitiveComponent Object Reference") (OtherBodyIndex :type Integer) (bFromSweep :type Boolean) (SweepResult :type "HitResult Structure (by ref)"))
  (if (== OtherActor (`GameplayStatics.GetPlayerPawn` 0))
    (bind _asfirst_person_character (cast `/Game/FirstPersonBP/Blueprints/FirstPersonCharacter` OtherActor))
    (`/Game/FirstPersonBP/Blueprints/FirstPersonCharacter.HurtFunction` _asfirst_person_character 5)
    (`self.DisableWeaponTrigger`)))

(fn `ActivateAntiGravity`
  (bind _mesh (`self.Mesh`))
  (if (not (`self.AntiGravity`))
    (`ActorComponent.Deactivate` (`self.CharacterMovement`)) ; Decativate Movement Component
    (`self.K2_AddActorWorldOffset` self (0.0 0.0 300.0) false true)
    (`PrimitiveComponent.SetEnableGravity` (`self.Mesh`) false)
    (`PrimitiveComponent.SetCollisionEnabled` _mesh "QueryAndPhysics")
    (`PrimitiveComponent.SetSimulatePhysics` _mesh true)
    (`ActorComponent.Deactivate` (`self.CharacterMovement`)) ; Decativate Movement Component
    (set `self.AntiGravity` true)))

(fn `ActivateFreeze`
  (set `SkeletalMeshComponent.bPauseAnims` true (`self.Mesh`))
  (`BrainComponent.StopLogic` (`AIController.BrainComponent` (`AIBlueprintHelperLibrary.GetAIController` self)) "Boi be frozen as shit")
  (set `self.Frozen` true)
  (`PrimitiveComponent.SetMaterial` (`self.Mesh`) 0 "/Game/SteamyRobots/Content/M_UE4Man_Body1_Inst_Freeze.M_UE4Man_Body1_Inst_Freeze"))

(fn `DeactivateAntiGravity`
  (bind _mesh (`self.Mesh`))
  (`PrimitiveComponent.SetSimulatePhysics` _mesh false)
  (`PrimitiveComponent.SetCollisionEnabled` _mesh "NoCollision")
  (`PrimitiveComponent.SetCollisionEnabled` (`self.Sword`) "NoCollision")
  (`SceneComponent.K2_AttachToComponent` (`self.Sword`) (`self.Mesh`) "SwordSocket" "SnapToTarget" "SnapToTarget" "KeepRelative" true)
  (`SceneComponent.K2_AttachToComponent` (`self.Mesh`) (`self.CapsuleComponent`) "None" "SnapToTarget" "SnapToTarget" "KeepRelative" true)
  (`SceneComponent.K2_SetRelativeTransform` (`self.Mesh`) (`KismetMathLibrary.MakeTransform` (0.0 0.0 -97.0) (struct :`Yaw` 270.0)) false true)
  (`ActorComponent.Activate` (`self.CharacterMovement`) true) ; Activate Movement Component
  (set `self.AntiGravity` false))

(fn `DeactivateFreeze`
  (set `SkeletalMeshComponent.bPauseAnims` false (`self.Mesh`))
  (`BrainComponent.RestartLogic` (`AIController.BrainComponent` (`AIBlueprintHelperLibrary.GetAIController` self)))
  (set `self.Frozen` false)
  (`PrimitiveComponent.SetMaterial` (`self.Mesh`) 0 "/Game/SteamyRobots/Content/M_UE4Man_Body1_Inst.M_UE4Man_Body1_Inst"))

(fn `HurtFunction`
  (params (Damage :type Integer))
  (bind _health (`self.Health`))
  (bind _asfirst_person_character (cast `/Game/FirstPersonBP/Blueprints/FirstPersonCharacter` (`GameplayStatics.GetPlayerCharacter` 0)))
  (`GameplayStatics.PlaySoundAtLocation` "/Game/Stuff/Sounds/HitSound.HitSound" (`SceneComponent.K2_GetComponentLocation` (`/Game/FirstPersonBP/Blueprints/FirstPersonCharacter.Mesh_Assault` _asfirst_person_character)) (struct) 1.0 1.0 0.0 (`self.NewVar_0`))
  (set `self.Health` (- _health Damage))
  (if (<= _health 0)
    (set `self.IsAlive` false)
    (bind _asfirst_person_character_2 (cast `/Game/FirstPersonBP/Blueprints/FirstPersonCharacter` (`GameplayStatics.GetPlayerCharacter` 0)))
    (`/Game/FirstPersonBP/Blueprints/FirstPersonCharacter.AddCurrency` _asfirst_person_character_2 100)
    (bind _asfirst_person_game_mode (cast `/Game/FirstPersonBP/Blueprints/FirstPersonGameMode` (`GameplayStatics.GetGameMode`)))
    (bind _spawnercontroller (`/Game/FirstPersonBP/Blueprints/FirstPersonGameMode.SpawnerController` _asfirst_person_game_mode))
    (bind _alivebots (`/Game/SteamyRobots/Ai-stuff/SpawnerController.AliveBots` _spawnercontroller))
    (set `/Game/SteamyRobots/Ai-stuff/SpawnerController.AliveBots` (- _alivebots 1) _spawnercontroller)
    (`/Engine/EditorBlueprintResources/StandardMacros.DecrementInt` (`/Game/SteamyRobots/Ai-stuff/SpawnerController.RealAliveBots` _spawnercontroller)
      (:`  `
        (if (== _alivebots 0)
          (`/Game/SteamyRobots/Ai-stuff/SpawnerController.StopWave` _spawnercontroller))
        (`/Game/SteamyRobots/Ai-stuff/MeleeBotSpawner.DeleteKilledMob` (`self.Spawner`) self)))))

(fn `UserConstructionScript`)